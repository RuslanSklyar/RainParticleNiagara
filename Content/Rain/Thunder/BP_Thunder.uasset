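; Lightning actor that loops a distant strike roughly every six seconds, with thunder audio and a screen flash.
; Each strike moves the actor far ahead of the player's view with random sideways offset, yawed to face the player.
; A timeline drives the bolt plane's Y and Emission material parameters before it is hidden.
; The flash briefly raises manual post-process exposure compensation, then restores the original value.
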(event `self.ReceiveBeginPlay`
  (bind _postprocess (`self.PostProcess`))
  (`KismetSystemLibrary.Delay` 6.0 :!label _label)
  (`self.Strike`)
  (`KismetSystemLibrary.Delay` 0.2)
  (bind _output_get (set `self.OriginalExposure Compensation` (`.AutoExposureBias` (break `PostProcessSettings` (`PostProcessVolume.Settings` _postprocess)))))
  (set `PostProcessVolume.Settings` (make `PostProcessSettings` :`AutoExposureMethod` "AEM_Manual" :`AutoExposureBias` 12.0) _postprocess)
  (`KismetSystemLibrary.Delay` 0.2)
  (set `PostProcessVolume.Settings` (make `PostProcessSettings` :`AutoExposureMethod` "AEM_Manual" :`AutoExposureBias` _output_get) (`self.PostProcess`))
  (goto _label))

(event `Strike`
  (bind _returnvalue (`Controller.GetControlRotation` (`GameplayStatics.GetPlayerController` 0)))
  (bind _returnvalue_2 (`self.K2_GetActorLocation` (`GameplayStatics.GetPlayerCharacter` 0)))
  (bind _returnvalue_3 (+ (* (`KismetMathLibrary.GetForwardVector` _returnvalue) (`KismetMathLibrary.RandomFloatInRange` 100000.0 100000.0)) _returnvalue_2 (* (`KismetMathLibrary.GetRightVector` _returnvalue) (`KismetMathLibrary.RandomFloatInRange` -3000.0 3000.0)) (0.0 0.0 500.0)))
  (bind (_returnvalue_roll _returnvalue_pitch _returnvalue_yaw) (`KismetMathLibrary.BreakRotator` (`KismetMathLibrary.FindLookAtRotation` _returnvalue_3 _returnvalue_2)))
  (`self.K2_SetActorLocationAndRotation` _returnvalue_3 (`KismetMathLibrary.MakeRotator` 0.0 0.0 _returnvalue_yaw))
  (`GameplayStatics.PlaySound2D` "/Game/Rain/Thunder/fonoteca-raskat-groma__online-audio-converter_com_.fonoteca-raskat-groma__online-audio-converter_com_" 1.0 1.0 0.0 null null)
  (`SceneComponent.SetVisibility` (`self.Plane`) true false)
  (bind (_direction _y) (`Timeline|Timeline_0` :!via `PlayFromStart`)
    (:`Update`
      (`MeshComponent.SetScalarParameterValueOnMaterials` (`self.Plane`) "Y" _y)
      (`MeshComponent.SetScalarParameterValueOnMaterials` (`self.Plane`) "Emission" (* (+ _y 1.0) 10.0))
      (`KismetSystemLibrary.Delay` 0.8)
      (`SceneComponent.SetVisibility` (`self.Plane`) false false))))

(fn `UserConstructionScript`)